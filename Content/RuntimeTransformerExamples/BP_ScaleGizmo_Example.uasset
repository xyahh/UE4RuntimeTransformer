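; Example scale gizmo for runtime transforming that highlights the handle mesh of the active transform domain.
; On BeginPlay it binds to the gizmo state change event, which maps the current axis, plane or XYZ domain to its mesh.
; Each change restores the previous mesh's cached materials, then caches the new mesh's materials and applies the selection material to every slot.
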(event `self.ReceiveBeginPlay`
  (add `BaseGizmo.OnGizmoStateChange` (delegate `OnGizmoStateChange_Event`)))

(event `OnGizmoStateChange_Event`
  (params (GizmoType :type "ETransformationType Enum" :default "TT_None") (bTransformInProgress :type Boolean) (CurrentDomain :type "ETransformationDomain Enum" :default "TD_None"))
  (bind _selectedmesh (`self.SelectedMesh`))
  (`/Engine/EditorBlueprintResources/StandardMacros.IsValid` (`self.SelectedMesh`)
    (:`Is Valid`
      (`|ExecutionSequence`
        (:`then_0`
          ;[1 1 1] Before Selecting a New Mesh, set the currently Selected Mesh back to its original state
          (for _index (range (`PrimitiveComponent.GetNumMaterials` (`self.SelectedMesh`)))
            (`PrimitiveComponent.SetMaterial` (`self.SelectedMesh`) _index (`|GetArrayItem` (`self.Original Materials`) _index))))
        (:`then_1`
          (switch `ETransformationDomain` CurrentDomain :!label _label
            (:`TD_X_Axis`
              ;[1 1 1] Check which is going to be Next Selected Mesh
              (set `self.SelectedMesh` (`self.X_Mesh`)))
            (:`TD_Y_Axis`
              (set `self.SelectedMesh` (`self.Y_Mesh`)))
            (:`TD_Z_Axis`
              (set `self.SelectedMesh` (`self.Z_Mesh`)))
            (:`TD_XY_Plane`
              (set `self.SelectedMesh` (`self.XY_Mesh`)))
            (:`TD_YZ_Plane`
              (set `self.SelectedMesh` (`self.YZ_Mesh`)))
            (:`TD_XZ_Plane`
              (set `self.SelectedMesh` (`self.XZ_Mesh`)))
            (:`TD_XYZ`
              (set `self.SelectedMesh` (`self.XYZ_Mesh`))))
          (`KismetArrayLibrary.Array_Clear` (`self.Original Materials`))
          ;[1 1 1] Save each Material by Index
          (for _index_2 (range (`PrimitiveComponent.GetNumMaterials` _selectedmesh))
            (`KismetArrayLibrary.Array_Add` (`self.Original Materials`) (`PrimitiveComponent.GetMaterial` _selectedmesh _index_2))
            (`PrimitiveComponent.SetMaterial` _selectedmesh _index_2 (`self.Material for Selection`))))))
    (:`Is Not Valid`
      (goto _label))))

(fn `UserConstructionScript`)